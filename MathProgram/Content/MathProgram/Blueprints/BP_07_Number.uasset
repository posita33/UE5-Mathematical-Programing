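; BP_07_Number is a Blueprint from a math exercise folder that prints the value of Pi on BeginPlay.
; The event graph converts the Pi constant to a string and passes it to PrintString.
; Unconnected leftover nodes build arithmetic expressions with variables, division and MultiplyByPi, but none of them execute.
; The overlap and Tick events are disabled, and the construction script is empty.
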(event `self.ReceiveBeginPlay`
  (`KismetSystemLibrary.PrintString` (`KismetStringLibrary.Conv_DoubleToString` (`KismetMathLibrary.GetPI`))))

(fn `UserConstructionScript`)