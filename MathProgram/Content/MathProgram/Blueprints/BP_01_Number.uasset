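; Math demo actor that shows a labeled, colored sphere and reports its position along the Y axis as a number and its absolute value.
; The construction script applies DispText to the TextRender and the Color variable to both the text and the sphere's material parameter.
; On BeginPlay it prints the actor's Y location and then its absolute value on screen in the same color, with Japanese labels.
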(event `self.ReceiveBeginPlay`
  (bind (_returnvalue_x _returnvalue_y) (`KismetMathLibrary.BreakVector` (`self.K2_GetActorLocation`)))
  (`|ExecutionSequence`
    (:`then_0`
      ;[1 1 1] 位置
      (`KismetSystemLibrary.PrintString` (`KismetStringLibrary.Concat_StrStr` "位置：" (`KismetStringLibrary.Conv_DoubleToString` _returnvalue_y)) true true (`self.Color`) 10.0))
    (:`then_1`
      ;[1 1 1] 絶対値
      (`KismetSystemLibrary.PrintString` (`KismetStringLibrary.Concat_StrStr` "絶対値：" (`KismetStringLibrary.Conv_DoubleToString` (`KismetMathLibrary.Abs` _returnvalue_y))) true true (`self.Color`) 10.0))))

(fn `UserConstructionScript`
  (bind _color (`self.Color`))
  (bind (_r _g _b) (`KismetMathLibrary.BreakColor` _color))
  (bind (_b_2 _g_2 _r_2 _a) (break `Color` (`KismetMathLibrary.Conv_LinearColorToColor` _color)))
  ;[1 1 1] Text
  (`TextRenderComponent.K2_SetText` (`self.TextRender`) (`self.DispText`))
  ;[1 1 1] Color
  (`MeshComponent.SetVectorParameterValueOnMaterials` (`self.Sphere`) "Color" (`KismetMathLibrary.MakeVector` _r _g _b))
  (`TextRenderComponent.SetTextRenderColor` (`self.TextRender`) (make `Color` _b_2 _g_2 _r_2 _a)))